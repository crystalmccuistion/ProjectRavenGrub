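; BPC_WeaponManager is a character component that swaps the owner's animation blueprint to match the weapon equipped in the main hand.
; On BeginPlay it caches the owning BP_Character_Base with its inventory and equipment managers, then binds to the equipment-changed event.
; The change handler applies the AnimClass from the spawned weapon's WeaponInfo to the mesh, or DefaultAnimClass when the main-hand slot is empty.
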(event `self.ReceiveBeginPlay`
  (bind _asbp_character_base (cast `/Game/Characters/BP_Character_Base` (`self.GetOwner`)))
  (set `self.Owner` _asbp_character_base)
  (set `self.InventoryManager` (`Actor.GetComponentByClass` _asbp_character_base "/Game/InventorySystem/BPC_InventoryManager.BPC_InventoryManager_C"))
  (bind _output_get (set `self.EquipmentManager` (`Actor.GetComponentByClass` _asbp_character_base "/Game/EquipmentSystem/BPC_EquipmentManager.BPC_EquipmentManager_C")))
  (add `/Game/EquipmentSystem/BPC_EquipmentManager.OnEquipmentChanged` _output_get (`|CreateDelegate` :!event `HandleOnEquipmentChanged`)))

(event `HandleOnEquipmentChanged`
  (bind _equipmentmanager (`self.EquipmentManager`)
    (:`then`
      (bind _equipment (`/Game/EquipmentSystem/BPC_EquipmentManager.FindEquipmentInSlot` _equipmentmanager (struct :`TagName` "Equipment.Slot.MainHand")))
      (`/Engine/EditorBlueprintResources/StandardMacros.IsValid` _equipment
        (:`Is Valid`
          (bind _spawnedequipmentactor (`EquipmentInstance.SpawnedEquipmentActor` _equipment)
            (:`then`
              (bind _asbp_weapon_base (cast `/Game/WeaponSystem/BP_Weapon_Base` _spawnedequipmentactor))
              (`SkeletalMeshComponent.SetAnimInstanceClass` (`Character.Mesh` (`self.Owner`)) (`.AnimClass_9_F1E595E54D2B6CE14586428FC4ADF4BC` (break `/Game/WeaponSystem/S_WeaponInfo` (`/Game/WeaponSystem/BP_Weapon_Base.WeaponInfo` _asbp_weapon_base)))))
            (:`else`)))
        (:`Is Not Valid`
          (`SkeletalMeshComponent.SetAnimInstanceClass` (`Character.Mesh` (`self.Owner`)) (`self.DefaultAnimClass`)))))
    (:`else`)))