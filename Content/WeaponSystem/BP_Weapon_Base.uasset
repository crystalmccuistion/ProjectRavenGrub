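; Base weapon Blueprint that performs hit detection on pawns and applies a supplied Gameplay Effect spec to them.
; HitScanStart clears the hit list and starts a looping ~30 Hz timer for sphere traces between two weapon points, until HitScanEnd.
; Each target with an Ability System Component is hit once per window, skipping the instigator and Status.Invincible tags.
; Each hit triggers a brief hit-stop through global time dilation.
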(event `HitScan`
  (bind _outhits (`KismetSystemLibrary.SphereTraceMultiForObjects` (`SceneComponent.K2_GetComponentLocation` (`self.TraceStart`)) (`SceneComponent.K2_GetComponentLocation` (`self.TraceEnd`)) (`self.HitScanRadius`) (`|MakeArray` "ObjectTypeQuery3" :!type "EObjectTypeQuery Enum") false (`|MakeArray` (`self.Instigator`) :!type "Actor Object Reference") "None" true (struct :`R` 1.0 :`A` 1.0) (struct :`G` 1.0 :`A` 1.0) 0.0))
  (for _array_element _outhits
    (bind _output_get (set `self.FoundHitActor` (`.HitActor` (`GameplayStatics.BreakHitResult` _array_element))))
    (`/Engine/EditorBlueprintResources/StandardMacros.IsValid` (`AbilitySystemBlueprintLibrary.GetAbilitySystemComponent` _output_get)
      (:`Is Valid`
        (if (and (not (`KismetArrayLibrary.Array_Contains` (`self.PreviouslyHitActors`) (`self.FoundHitActor`))) (not (`BlueprintGameplayTagLibrary.HasTag` (`/Game/Blueprints/BPC_TagManager.TagContainer` (`self.GetComponentByClass` (`self.FoundHitActor`) "/Game/Blueprints/BPC_TagManager.BPC_TagManager_C")) (struct :`TagName` "Status.Invincible"))))
          (`KismetArrayLibrary.Array_AddUnique` (`self.PreviouslyHitActors`) (`self.FoundHitActor`))
          (`AbilitySystemComponent.BP_ApplyGameplayEffectSpecToSelf` (`AbilitySystemBlueprintLibrary.GetAbilitySystemComponent` (`self.FoundHitActor`)) (`self.GameplayEffectSpecHandle`))
          (`self.DoHitStopEffect`))))))

(event `DoHitStopEffect`
  (`GameplayStatics.SetGlobalTimeDilation` 0.1)
  (`KismetSystemLibrary.Delay` 0.01)
  (`GameplayStatics.SetGlobalTimeDilation` 1.0))

(event `HitScanStart`
  (params (GameplayEffectSpecHandle :type "GameplayEffectSpecHandle Structure"))
  (set `self.GameplayEffectSpecHandle` GameplayEffectSpecHandle)
  (`KismetArrayLibrary.Array_Clear` (`self.PreviouslyHitActors`))
  (bind _returnvalue (`KismetSystemLibrary.K2_SetTimerDelegate` (`|CreateDelegate` :!event `HitScan`) 0.033333 true))
  (set `self.HitScanTimer` _returnvalue))

(event `HitScanEnd`
  (`KismetSystemLibrary.K2_ClearAndInvalidateTimerHandle` (`self.HitScanTimer`)))

(fn `UserConstructionScript`)