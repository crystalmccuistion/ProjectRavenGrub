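; BP_GroundMessage is a level actor that shows a text message on the player's HUD while the player pawn is within range.
; Overlap begin and end call Activate and Deactivate, and BeginPlay waits one frame to catch a player already inside InteractableRadius.
; Activate reaches the HUD through BP_PlayerController, sets MessageText on WMessagePanel and plays its show animation; Deactivate plays the hide animation.
; Its interact prompt getter returns an empty string.
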(event `self.ReceiveBeginPlay`
  (`KismetSystemLibrary.DelayUntilNextFrame`)
  (if (`KismetArrayLibrary.Array_IsNotEmpty` (`PrimitiveComponent.GetOverlappingActors` (`self.InteractableRadius`) "/Game/Characters/BP_Player.BP_Player_C"))
    (`self.Activate`)))

(event `self.ReceiveActorBeginOverlap`
  (params (OtherActor :type "Actor Object Reference"))
  (if (== OtherActor (`GameplayStatics.GetPlayerPawn` 0))
    (`self.Activate`)))

(event `self.ReceiveActorEndOverlap`
  (params (OtherActor :type "Actor Object Reference"))
  (if (== OtherActor (`GameplayStatics.GetPlayerPawn` 0))
    (`self.Deactivate`)))

(fn `Activate`
  (bind _asbp_player_controller (cast `/Game/Blueprints/CoreSystems/BP_PlayerController` (`GameplayStatics.GetPlayerController` 0)))
  (bind _playerhudref (`/Game/Blueprints/CoreSystems/BP_PlayerController.PlayerHUDRef` _asbp_player_controller))
  (bind _w_messagepanel (`/Game/UI/Widgets/Screens/Screen_HUD.W_MessagePanel` _playerhudref))
  (`Widget.SetVisibility` _w_messagepanel "Visible")
  (set `TextBlock.Text` (`self.MessageText`) (`/Game/UI/Widgets/W_Message.MessageText` _w_messagepanel))
  (`UserWidget.PlayAnimation` _playerhudref (`/Game/UI/Widgets/Screens/Screen_HUD.ShowMessagePanel` _playerhudref) 0.0 1 "Forward" 1.0 false))

(fn `Deactivate`
  (bind _asbp_player_controller (cast `/Game/Blueprints/CoreSystems/BP_PlayerController` (`GameplayStatics.GetPlayerController` 0)))
  (bind _playerhudref (`/Game/Blueprints/CoreSystems/BP_PlayerController.PlayerHUDRef` _asbp_player_controller))
  (`UserWidget.PlayAnimation` _playerhudref (`/Game/UI/Widgets/Screens/Screen_HUD.HideMessagePanel` _playerhudref) 0.0 1 "Forward" 1.0 false))

(fn `GetInteractPrompt`
  (returns (PromptText :type Text))
  (return ""))

(fn `GetInteractSocket`
  (returns (InteractSocket :type "SceneComponent Object Reference"))
  (return (`self.InteractSocket`)))

(fn `UserConstructionScript`)