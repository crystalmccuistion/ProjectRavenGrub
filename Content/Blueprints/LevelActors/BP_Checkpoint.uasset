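; BP_Checkpoint is an interactable level checkpoint that sets the player's spawnpoint and offers rest.
; It counts as active when the save game's PlayerStartTag matches its PlayerStart, which switches the prompt between activate and rest.
; Activation refills health potions, fully heals, stores the tag and announces the new spawnpoint.
; Resting refills potions, saves the player through BPC_WorldPersistence and respawns them through the player controller.
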(event `/Game/Blueprints/BPI_Interactable.Interact`
  (params (Interactor :type "Actor Object Reference"))
  (if (`self.IsActive`)
    (`self.StartPlayerRest`)
    (else
      (`self.ActivateCheckpoint` Interactor))))

(event `SetPlayerSpawnpoint`
  (bind _savegameobject (message `/Game/SaveSystem/BPI_SaveAndLoadManager.GetSaveGameObject` (`GameplayStatics.GetGameInstance`)))
  (set `/Game/SaveSystem/BP_SaveGame.PlayerStartTag` (`PlayerStart.PlayerStartTag` (`self.PlayerStart`)) _savegameobject))

(event `HealPlayer`
  (params (Interactor :type "Actor Object Reference"))
  (`/Engine/EditorBlueprintResources/StandardMacros.IsValid` Interactor
    (:`Is Valid`
      (bind _asbp_player (cast `/Game/Characters/BP_Player` Interactor))
      (`DamageableInterface.Heal` _asbp_player (`DamageSystemComponent.GetMaxHealth` (`/Game/Characters/BP_Character_Base.DamageSystem` _asbp_player)) self))))

(fn `ActivateCheckpoint`
  (params (Interactor :type "Actor Object Reference"))
  (bind _asbp_player (cast `/Game/Characters/BP_Player` Interactor)
    (:`then`
      (`/Game/InventorySystem/BPC_InventoryManager.SetItemCount` (`/Game/Characters/BP_Character_Base.BPC_InventoryManager` _asbp_player) "/Game/InventorySystem/Items/Item_HealthPotion.Item_HealthPotion_C" 5))
    (:`CastFailed`
      _))
  (`self.HealPlayer` Interactor)
  (`self.SetPlayerSpawnpoint`)
  (`GameplayStatics.PlaySoundAtLocation` "/Game/Sounds/SFX_ActivateCheckpoint_Cue.SFX_ActivateCheckpoint_Cue" (`self.K2_GetActorLocation` self) (struct) 1.0 1.0 0.0 null null null null)
  (bind _returnvalue (`|GenericCreateObject` "/Game/UI/Widgets/W_Display_Announcement.W_Display_Announcement_C" "SPAWNPOINT SET"))
  (`UserWidget.AddToViewport` _returnvalue 0))

(fn `GetInteractPrompt`
  (returns (PromptText :type Text))
  (if (`self.IsActive`)
    (return "Rest")
    (else
      (return "Activate checkpoint"))))

(fn `GetInteractSocket`
  (returns (InteractSocket :type "SceneComponent Object Reference"))
  (return (`self.InteractSocket`)))

(fn `GetSaveGameObject`
  (returns (SaveGameObject :type "/Game/SaveSystem/BP_SaveGame Object Reference"))
  (return null))

(fn `GetSpawnpointTransform`
  (returns (SpawnpointTransform :type "Transform Structure"))
  (return (`SceneComponent.K2_GetComponentToWorld` (`self.Spawnpoint`))))

(fn `IsActive`
  (returns (`Return Value` :type Boolean))
  (bind _savegameobject (message `/Game/SaveSystem/BPI_SaveAndLoadManager.GetSaveGameObject` (`GameplayStatics.GetGameInstance`)))
  (if (== (`/Game/SaveSystem/BP_SaveGame.PlayerStartTag` _savegameobject) (`PlayerStart.PlayerStartTag` (`self.PlayerStart`)))
    (return true)
    (else
      (return false))))

(fn `StartPlayerRest`
  (bind _returnvalue (`self.GetComponentByClass` (`GameplayStatics.GetGameMode`) "/Game/SaveSystem/BPC_WorldPersistence.BPC_WorldPersistence_C"))
  (`GameplayStatics.PlaySoundAtLocation` "/Game/UI/Sound/UI_Confirm_Cue.UI_Confirm_Cue" (`self.K2_GetActorLocation` self) (struct) 1.0 1.0 0.0 null null null null)
  (bind _asbp_player (cast `/Game/Characters/BP_Player` (`GameplayStatics.GetPlayerPawn` 0))
    (:`then`
      (`/Game/InventorySystem/BPC_InventoryManager.SetItemCount` (`/Game/Characters/BP_Character_Base.BPC_InventoryManager` _asbp_player) "/Game/InventorySystem/Items/Item_HealthPotion.Item_HealthPotion_C" 5)
      (`/Engine/EditorBlueprintResources/StandardMacros.IsValid` _returnvalue
        (:`Is Valid`
          (`/Game/SaveSystem/BPC_WorldPersistence.HandleSavePlayer` _returnvalue (`GameplayStatics.GetPlayerController` 0))
          (bind _asbp_player_controller (cast `/Game/Blueprints/CoreSystems/BP_PlayerController` (`GameplayStatics.GetPlayerController` 0))))
        (:`Is Not Valid`
          _)))
    (:`CastFailed`
      _))
  (`/Game/Blueprints/CoreSystems/BP_PlayerController.RespawnPlayer` _asbp_player_controller))

(fn `UserConstructionScript`)