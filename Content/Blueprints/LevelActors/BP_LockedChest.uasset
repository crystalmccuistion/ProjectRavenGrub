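; BP_LockedChest is an interactable chest that takes a lockpick to unlock.
; On interact, it searches the interactor's inventory component for lockpicks and checks each one's limited-use item fragment.
; The first usable pick loses a use, plays a success cue and blocks further success; no opening or loot logic follows.
; Failures call a sound handler with no sound set, firing once per rejected pick inside the loop.
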(event `/Game/Blueprints/BPI_Interactable.Interact`
  (params (Interactor :type "Actor Object Reference"))
  (bind _returnvalue (`self.GetComponentByClass` Interactor "/Game/InventorySystem/BPC_InventoryManager.BPC_InventoryManager_C"))
  (`/Engine/EditorBlueprintResources/StandardMacros.IsValid` _returnvalue
    (:`Is Valid`
      (bind _inventoryitems (`/Game/InventorySystem/BPC_InventoryManager.FindAllItems` _returnvalue "/Game/InventorySystem/Items/Item_Lockpick.Item_Lockpick_C"))
      (if (`KismetArrayLibrary.Array_IsNotEmpty` _inventoryitems)
        (for _array_element _inventoryitems
          (bind _iteminstance (break `/Game/InventorySystem/Types/S_InventoryItem` _array_element))
          (if (`/Game/InventorySystem/Fragments/BP_ItemFragment_LimitedUse.HasUsesLeft` (`ItemInstance.FindFragmentByClass` _iteminstance "/Game/InventorySystem/Fragments/BP_ItemFragment_LimitedUse.BP_ItemFragment_LimitedUse_C") _iteminstance)
            (if (not (`self.InteractionBlocked`))
              (`self.Handle Interact Succeed` _iteminstance)
              (break)
              (else
                _)))
          (`self.HandleInteractFail` :!label _label))
        (else
          (goto _label))))
    (:`Is Not Valid`
      (goto _label))))

(event `HandleInteractFail`
  (`GameplayStatics.PlaySoundAtLocation` null (`SceneComponent.K2_GetComponentLocation` (`self.StaticMesh`)) (struct) 1.0 1.0 0.0 null null null null))

(event `Handle Interact Succeed`
  (params (ItemInstance :type "ItemInstance Object Reference"))
  (set `self.InteractionBlocked` true)
  (`GameplayStatics.PlaySoundAtLocation` "/Game/Sounds/SFX_NewArea_Cue.SFX_NewArea_Cue" (`SceneComponent.K2_GetComponentLocation` (`self.StaticMesh`)) (struct) 1.0 1.0 0.0 null null null null)
  (`/Game/InventorySystem/Fragments/BP_ItemFragment_LimitedUse.DecrementUsesLeft` (`ItemInstance.FindFragmentByClass` ItemInstance "/Game/InventorySystem/Fragments/BP_ItemFragment_LimitedUse.BP_ItemFragment_LimitedUse_C") ItemInstance))

(fn `GetInteractPrompt`
  (returns (PromptText :type Text))
  (return ""))

(fn `GetInteractSocket`
  (returns (InteractSocket :type "SceneComponent Object Reference"))
  (return (`self.InteractSocket`)))

(fn `UserConstructionScript`)