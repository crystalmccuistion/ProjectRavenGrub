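; BP_PickupItem is an interactable world pickup that adds its item snapshot to the player's inventory, plays a sound and destroys itself.
; The construction script sets the mesh from the item definition's world-representation fragment and assigns a persistent GUID when none is valid.
; On pickup it records that GUID in the save game's destroyed-actor list, and BeginPlay destroys any pickup already listed.
; Its interact prompt shows the item name, plus the count for stacks.
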(event `self.ReceiveBeginPlay`
  (bind _savegameobject (message `/Game/SaveSystem/BPI_SaveAndLoadManager.GetSaveGameObject` (`GameplayStatics.GetGameInstance`)))
  (`/Engine/EditorBlueprintResources/StandardMacros.IsValid` _savegameobject
    (:`Is Valid`
      (if (`KismetArrayLibrary.Array_Contains` (`/Game/SaveSystem/BP_SaveGame.DestroyedActors` _savegameobject) (`self.UniqueID`))
        (`self.K2_DestroyActor`)))))

(event `/Game/Blueprints/BPI_Interactable.Interact`
  (params (Interactor :type "Actor Object Reference"))
  (bind _returnvalue (`self.GetComponentByClass` (`GameplayStatics.GetPlayerPawn` 0) "/Game/InventorySystem/BPC_InventoryManager.BPC_InventoryManager_C"))
  (`/Engine/EditorBlueprintResources/StandardMacros.IsValid` _returnvalue
    (:`Is Valid`
      (`/Game/InventorySystem/BPC_InventoryManager.AddItem` _returnvalue (`self.InventoryItemSnapshot`))
      (`GameplayStatics.PlaySoundAtLocation` "/Game/Sounds/SFX_GetItem_Cue.SFX_GetItem_Cue" (`SceneComponent.K2_GetComponentLocation` (`self.InteractableRadius`)) (struct) 1.0 1.0 0.0 null null null null)
      (bind _savegameobject (message `/Game/SaveSystem/BPI_SaveAndLoadManager.GetSaveGameObject` (`GameplayStatics.GetGameInstance`)))
      (`/Engine/EditorBlueprintResources/StandardMacros.IsValid` _savegameobject
        (:`Is Valid`
          (`KismetArrayLibrary.Array_AddUnique` (`/Game/SaveSystem/BP_SaveGame.DestroyedActors` _savegameobject) (`self.UniqueID`)))
        (:`Is Not Valid`
          _))
      (`self.K2_DestroyActor`))))

(fn `GetInteractPrompt`
  (returns (PromptText :type Text))
  (bind (_itemdefinition _count) (break `/Game/InventorySystem/Types/S_InventoryItemSnapshot` (`self.InventoryItemSnapshot`)))
  (bind _itemname (defaults `Object` _itemdefinition))
  (if (> _count 1)
    (return (`|FormatText` "Pick up {name} x{count}" _itemname _count))
    (else
      (return (`|FormatText` "Pick up {name}" _itemname)))))

(fn `GetInteractSocket`
  (returns (InteractSocket :type "SceneComponent Object Reference"))
  (return (`self.InteractSocket`)))

(fn `UserConstructionScript`
  (bind _inventoryitemsnapshot_itemdefinition (break `/Game/InventorySystem/Types/S_InventoryItemSnapshot` (`self.InventoryItemSnapshot`)))
  (bind _returnvalue (`ItemDefinition.FindFragmentByClass` _inventoryitemsnapshot_itemdefinition "/Script/ProjectRavenGrub.InventoryItemFragment_WorldRepresentation"))
  (`|ExecutionSequence`
    (:`then_0`
      ; Set Static Mesh
      (`/Engine/EditorBlueprintResources/StandardMacros.IsValid` _returnvalue
        (:`Is Valid`
          (`StaticMeshComponent.SetStaticMesh` (`self.StaticMesh`) (`InventoryItemFragment_WorldRepresentation.ItemMesh` _returnvalue))
          (`self.SetActorHiddenInGame` false))))
    (:`then_1`
      (if (not (`KismetGuidLibrary.IsValid_Guid` (`self.UniqueID`)))
        (set `self.UniqueID` (`KismetGuidLibrary.NewGuid`))))))