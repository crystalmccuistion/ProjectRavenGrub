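; Game mode for RavenGrub that handles player death, respawn and save-based spawn placement.
; On player death it waits briefly, then reloads the current level.
; ChoosePlayerStart reads the game instance's save, using the checkpoint PlayerStart with the saved tag if the player died, otherwise spawning a temporary PlayerStart at the saved transform.
; One tick after a player restarts, the world persistence component loads that player.
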(event `self.ReceiveBeginPlay`
  (bind _asbp_player (cast `/Game/Characters/BP_Player` (`GameplayStatics.GetPlayerPawn` 0)))
  (add `/Game/Characters/BP_Player.OnPlayerDeath` _asbp_player (delegate `HandleOnPlayerDeath`)))

(event `HandleOnPlayerDeath`
  (`KismetSystemLibrary.Delay` 10.0)
  (`self.RespawnPlayer`))

(event `self.K2_OnRestartPlayer`
  (params (NewPlayer :type "Controller Object Reference"))
  (`KismetSystemLibrary.DelayUntilNextTick`)
  (`/Game/SaveSystem/BPC_WorldPersistence.HandleLoadPlayer` (`self.BPC_WorldPersistence`) NewPlayer))

(fn `ChoosePlayerStart`
  (params (Player :type "Controller Object Reference"))
  (returns (ReturnValue :type "Actor Object Reference"))
  (bind _savegameobject (message `/Game/SaveSystem/BPI_SaveAndLoadManager.GetSaveGameObject` (`GameplayStatics.GetGameInstance`)))
  (bind (_playerstatesnapshot_currentstamina _playerstatesnapshot_currenthealth _playerstatesnapshot_transform _playerstatesnapshot_isdead) (break `/Game/SaveSystem/S_PlayerStateSnapshot` (`/Game/SaveSystem/BP_SaveGame.PlayerStateSnapshot` _savegameobject)))
  (if _playerstatesnapshot_isdead
    ; Player is dead; reload from last checkpoint
    (bind _outactors (`GameplayStatics.GetAllActorsOfClass` "/Script/Engine.PlayerStart"))
    (for _array_element _outactors
      (if (== (`PlayerStart.PlayerStartTag` _array_element) (`/Game/SaveSystem/BP_SaveGame.PlayerStartTag` _savegameobject))
        (return _array_element)))
    (else
      ; Player is alive; create temp Player Start actor and use it
      (bind _returnvalue (`|SpawnActorFromClass` "/Script/Engine.PlayerStart" _playerstatesnapshot_transform "Undefined" "MultiplyWithRoot" null null))
      (return _returnvalue))))

(fn `GetSaveGameObject`
  (returns (SaveGameObject :type "/Game/SaveSystem/BP_SaveGame Object Reference"))
  (return null))

(fn `RespawnPlayer`
  (bind _returnvalue (`GameplayStatics.GetCurrentLevelName` true))
  (`GameplayStatics.OpenLevel` (`KismetStringLibrary.Conv_StringToName` _returnvalue)))

(fn `UserConstructionScript`)