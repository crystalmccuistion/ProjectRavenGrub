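; Combat component for BP_Character_Base owners that runs sword combos and dodge rolls, gated by Status.Busy gameplay tags.
; Repeated attack input queues combos, which montage notifies continue or stop; players pay stamina.
; Dodges choose directional montages when strafing and grant timed invincibility, while Tick aims control rotation at any valid target.
; Hurtbox trace events are empty; their sphere-trace, damage and hit-stop logic is disconnected and never runs.
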(event `self.ReceiveBeginPlay`
  (bind _asbp_character_base (cast `/Game/Characters/BP_Character_Base` (`self.GetOwner`)))
  (set `self.OwnerRef` _asbp_character_base))

(event `self.ReceiveTick`
  (params (DeltaSeconds :type "Float (single-precision)"))
  (`self.FaceTarget`))

(event `Light Attack`
  (bind _tagcontainer (`/Game/Blueprints/BFL_TagHelpers.GetActorGameplayTagContainer` (`self.GetOwner`)))
  ; Attacks
  ;; Light attack
  (if (or (not (`BlueprintGameplayTagLibrary.HasTag` _tagcontainer (struct :`TagName` "Status.Busy"))) (`BlueprintGameplayTagLibrary.HasTag` _tagcontainer (struct :`TagName` "Status.Busy.Attacking")))
    (`/Game/Blueprints/BFL_TagHelpers.AddGameplayTagToActor` (`self.GetOwner`) (struct :`TagName` "Status.Busy.Attacking"))
    (if (not (`self.isAttacking`))
      (set `self.isAttacking` true)
      ;;; Animation
      (`GameplayStatics.PlaySoundAtLocation` "/Game/Sounds/SFX_SwordSwing_Cue.SFX_SwordSwing_Cue" (`Actor.K2_GetActorLocation` (`self.OwnerRef`)) (struct) 1.0 1.0 0.0 null null null null)
      (bind _asbp_player (cast `/Game/Characters/BP_Player` (`self.OwnerRef`))
        (:`then`
          (`/Game/Characters/BP_Player.SpendStamina` _asbp_player 20.0))
        (:`CastFailed`
          _))
      (`|PlayMontage` (`Character.Mesh` (`self.OwnerRef`)) "/Game/Characters/Animations/Attacks/Doll_Attack_SwordCombo_Montage.Doll_Attack_SwordCombo_Montage"
        (:`OnCompleted`
          (set `self.isAttacking` false :!label _label)
          (`/Game/Blueprints/BFL_TagHelpers.RemoveGameplayTagFromActor` (`self.GetOwner`) (struct :`TagName` "Status.Busy.Attacking")))
        (:`OnInterrupted`
          (goto _label))
        (:`OnNotifyBegin`
          (if (and (`self.isComboing`) (`self.isAttacking`))
            (set `self.isComboing` false)
            (`GameplayStatics.PlaySoundAtLocation` "/Game/Sounds/SFX_SwordSwing_Cue.SFX_SwordSwing_Cue" (`Actor.K2_GetActorLocation` (`self.OwnerRef`)) (struct) 1.0 1.0 0.0 null null null null)
            (bind _asbp_player_2 (cast `/Game/Characters/BP_Player` (`self.OwnerRef`)))
            (`/Game/Characters/BP_Player.SpendStamina` _asbp_player_2 (`self.LightAttackStaminaCost`))
            (else
              (`AnimInstance.Montage_Stop` (`SkeletalMeshComponent.GetAnimInstance` (`Character.Mesh` (`self.OwnerRef`))) 0.2 "/Game/Characters/Animations/Attacks/Doll_Attack_SwordCombo_Montage.Doll_Attack_SwordCombo_Montage")
              (`/Game/Blueprints/BFL_TagHelpers.RemoveGameplayTagFromActor` (`self.GetOwner`) (struct :`TagName` "Status.Busy.Attacking"))))))
      (else
        (set `self.isComboing` true)))))

(event `Begin Hurtbox Trace`
  ; Attacks
  ;; Hurtbox Trace
  ;;; Start hurtbox trace
)

(event `Increment Hurtbox Trace`
  ; Attacks
  ;; Hurtbox Trace
  ;;; Increment hurtbox trace
)

(event `End Hurtbox Trace`
  ; Attacks
  ;; Hurtbox Trace
  ;;; End hurtbox trace
)

(event `Hit Stop`
  ; Attacks
  (`GameplayStatics.SetGlobalTimeDilation` 0.1)
  (`KismetSystemLibrary.Delay` 0.005)
  (`GameplayStatics.SetGlobalTimeDilation` 1.0))

(event `Dodge`
  ; Dodge
  (if (not (`BlueprintGameplayTagLibrary.HasTag` (`/Game/Blueprints/BFL_TagHelpers.GetActorGameplayTagContainer` (`self.GetOwner`)) (struct :`TagName` "Status.Busy")))
    (`/Game/Blueprints/BFL_TagHelpers.AddGameplayTagToActor` (`self.GetOwner`) (struct :`TagName` "Status.Busy.Dodging"))
    (`|ExecutionSequence`
      (:`then_0`
        (if (`self.IsStrafing`)
          (switch `int` (`KismetArrayLibrary.Array_Find` (`EnhancedInputSubsystemInterface.QueryKeysMappedToAction` (pcsubsystem `EnhancedInputLocalPlayerSubsystem` (`GameplayStatics.GetPlayerController` 0)) "/Game/Input/Actions/IA_Move.IA_Move") (`/Game/Characters/BP_Character_Base.GetMoveDirectionKey` (`self.OwnerRef`)))
            (:`Default`
              (set `self.MoveDirection` "NewEnumerator0"))
            (:`0`
              (set `self.MoveDirection` "NewEnumerator0"))
            (:`1`
              (set `self.MoveDirection` "NewEnumerator1"))
            (:`2`
              (set `self.MoveDirection` "NewEnumerator2"))
            (:`3`
              (set `self.MoveDirection` "NewEnumerator3")))
          (else
            (set `self.MoveDirection` "NewEnumerator0"))))
      (:`then_1`
        (`self.SnapCharacterRotationToMoveInput`)
        (`|PlayMontage` (`Character.Mesh` (`self.OwnerRef`)) (select `/Game/Blueprints/E_MovementDirection` (`self.MoveDirection`) :`NewEnumerator0` "/Game/Characters/Animations/Roll/Dodge_F_Montage_ChaserDoll.Dodge_F_Montage_ChaserDoll" :`NewEnumerator1` "/Game/Characters/Animations/Roll/Dodge_B_Montage_ChaserDoll.Dodge_B_Montage_ChaserDoll" :`NewEnumerator2` "/Game/Characters/Animations/Roll/Dodge_L_Montage_ChaserDoll.Dodge_L_Montage_ChaserDoll" :`NewEnumerator3` "/Game/Characters/Animations/Roll/Dodge_R_Montage_ChaserDoll.Dodge_R_Montage_ChaserDoll" :!type "AnimMontage Object Reference")
          (:`then`
            (message `/Game/Blueprints/BPI_Combat.BeginInvincibility` (`self.OwnerRef`))
            (`KismetSystemLibrary.Delay` 0.6)
            (message `/Game/Blueprints/BPI_Combat.EndInvincibility` (`self.OwnerRef`))
            (`/Game/Blueprints/BFL_TagHelpers.RemoveGameplayTagFromActor` (`self.GetOwner`) (struct :`TagName` "Status.Busy.Dodging")))))
      (:`then_2`
        (`GameplayStatics.PlaySoundAtLocation` "/Game/Sounds/SFX_MedRoll_Cue.SFX_MedRoll_Cue" (`Actor.K2_GetActorLocation` (`self.OwnerRef`)) (struct) 1.0 1.0 0.0 null null null null))
      (:`then_3`
        (bind _asbp_player (cast `/Game/Characters/BP_Player` (`self.OwnerRef`)))
        (`/Game/Characters/BP_Player.SpendStamina` _asbp_player (`self.DodgeStaminaCost`))))))

(fn `FaceTarget`
  (bind (_returnvalue_roll _returnvalue_pitch _returnvalue_yaw) (`KismetMathLibrary.BreakRotator` (`KismetMathLibrary.FindLookAtRotation` (`Actor.K2_GetActorLocation` (`self.OwnerRef`)) (`Actor.K2_GetActorLocation` (`self.TargetRef`)))))
  (`/Engine/EditorBlueprintResources/StandardMacros.IsValid` (`self.TargetRef`)
    (:`Is Valid`
      (`Controller.SetControlRotation` (`Pawn.GetController` (`self.OwnerRef`)) (`KismetMathLibrary.MakeRotator` _returnvalue_roll (+ _returnvalue_pitch -16.0) _returnvalue_yaw)))))

(fn `SnapCharacterRotationToMoveInput`
  (returns (Success :type Boolean))
  (bind _returnvalue (`Pawn.GetLastMovementInputVector` (`self.OwnerRef`)))
  (if (and (not (`KismetMathLibrary.Vector_IsZero` _returnvalue)) (not (`self.IsStrafing`)))
    (`Actor.K2_SetActorRotation` (`self.OwnerRef`) (`KismetMathLibrary.Conv_VectorToRotator` _returnvalue) false)
    (return true)
    (else
      (return false))))

(fn `SnapCharacterRotationToTarget`
  (params (TargetRef :type "Actor Object Reference")))