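; Blueprint function library of helpers for reading and editing gameplay tags on actors.
; Each function finds the actor's BPC_TagManager component and works on its TagContainer: one returns the container, the others add or remove a single tag.
; Actors without that component are handled silently, with an empty return or no change.
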(fn `AddGameplayTagToActor`
  (params (Actor :type "Actor Object Reference") (Tag :type "GameplayTag Structure"))
  (bind _returnvalue (`Actor.GetComponentByClass` Actor "/Game/Blueprints/BPC_TagManager.BPC_TagManager_C"))
  (`/Engine/EditorBlueprintResources/StandardMacros.IsValid` _returnvalue
    (:`Is Valid`
      (`BlueprintGameplayTagLibrary.AddGameplayTag` (`/Game/Blueprints/BPC_TagManager.TagContainer` _returnvalue) Tag))))

(fn `GetActorGameplayTagContainer`
  (params (ActorRef :type "Actor Object Reference"))
  (returns (TagContainer :type "GameplayTagContainer Structure"))
  (bind _returnvalue (`Actor.GetComponentByClass` ActorRef "/Game/Blueprints/BPC_TagManager.BPC_TagManager_C"))
  (`/Engine/EditorBlueprintResources/StandardMacros.IsValid` _returnvalue
    (:`Is Valid`
      (return (`/Game/Blueprints/BPC_TagManager.TagContainer` _returnvalue)))
    (:`Is Not Valid`
      (return))))

(fn `RemoveGameplayTagFromActor`
  (params (Actor :type "Actor Object Reference") (Tag :type "GameplayTag Structure"))
  (bind _returnvalue (`Actor.GetComponentByClass` Actor "/Game/Blueprints/BPC_TagManager.BPC_TagManager_C"))
  (`/Engine/EditorBlueprintResources/StandardMacros.IsValid` _returnvalue
    (:`Is Valid`
      (`BlueprintGameplayTagLibrary.RemoveGameplayTag` (`/Game/Blueprints/BPC_TagManager.TagContainer` _returnvalue) Tag))))