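; BP_Checkpoint is an interactable checkpoint that sets the player's respawn point.
; On Interact, it writes the world transform of its Spawnpoint component to the Spawnpoint stored in player 0's BP_ThirdPersonPlayerState.
; The update and activation sound occur only when that transform differs from the saved one, so repeat interactions do nothing.
; A getter exposes InteractSocket to other Blueprints.
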(event `/Game/Blueprints/BPI_Interactable.Interact`
  (bind _asbp_third_person_player_state (cast `/Game/ThirdPerson/Blueprints/BP_ThirdPersonPlayerState` (`GameplayStatics.GetPlayerState` 0)))
  (if (not (== (`/Game/ThirdPerson/Blueprints/BP_ThirdPersonPlayerState.Spawnpoint` _asbp_third_person_player_state) (`self.GetSpawnpointTransform`)))
    (set `/Game/ThirdPerson/Blueprints/BP_ThirdPersonPlayerState.Spawnpoint` (`self.GetSpawnpointTransform`) _asbp_third_person_player_state)
    (`GameplayStatics.PlaySoundAtLocation` "/Game/Sound/SFX_ActivateCheckpoint_Cue.SFX_ActivateCheckpoint_Cue" (`self.K2_GetActorLocation` self) (struct) 1.0 1.0 0.0 null null null null)))

(fn `GetInteractSocket`
  (returns (InteractSocket :type "SceneComponent Object Reference"))
  (return (`self.InteractSocket`)))

(fn `GetSpawnpointTransform`
  (returns (SpawnpointTransform :type "Transform Structure"))
  (return (`SceneComponent.K2_GetComponentToWorld` (`self.Spawnpoint`))))

(fn `UserConstructionScript`)