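; World persistence component that saves and restores per-level dropped items and coordinates player saving and loading.
; Pickups tagged "DroppedItem" are snapshotted into the GameInstance's save object by level name, then respawned and retagged on BeginPlay.
; Player save records level state, delegates to inventory, equipment and BP_Player, then has the GameInstance save.
; Player load delegates to those three separately from level loading.
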(event `self.ReceiveBeginPlay`
  (`self.HandleLoadLevelState`))

(event `HandleSaveLevelState`
  ; Load/save world
  (bind _savegameobject (message `/Game/SaveSystem/BPI_SaveAndLoadManager.GetSaveGameObject` (`GameplayStatics.GetGameInstance`)))
  (`/Engine/EditorBlueprintResources/StandardMacros.IsValid` _savegameobject
    (:`Is Valid`
      (`KismetArrayLibrary.Array_Clear` (`self.DroppedItemsTemp`))
      (bind _outactors (`GameplayStatics.GetAllActorsOfClassWithTag` "/Game/InventorySystem/BP_PickupItem.BP_PickupItem_C" "DroppedItem"))
      (for _array_element _outactors
        (`KismetArrayLibrary.Array_Add` (`self.DroppedItemsTemp`) (make `/Game/SaveSystem/S_DroppedItemSnapshot` (`/Game/InventorySystem/BP_PickupItem.InventoryItemSnapshot` _array_element) (`Actor.GetTransform` _array_element))))
      (bind _returnvalue (`GameplayStatics.GetCurrentLevelName` true))
      (bind _savegameobject_2 (message `/Game/SaveSystem/BPI_SaveAndLoadManager.GetSaveGameObject` (`GameplayStatics.GetGameInstance`)))
      (`BlueprintMapLibrary.Map_Add` (`/Game/SaveSystem/BP_SaveGame.DroppedItemsByLevel` _savegameobject_2) _returnvalue (make `/Game/SaveSystem/S_DroppedItemSnapshotArray` (`self.DroppedItemsTemp`))))))

(event `HandleLoadLevelState`
  ; Load/save world
  (bind _savegameobject (message `/Game/SaveSystem/BPI_SaveAndLoadManager.GetSaveGameObject` (`GameplayStatics.GetGameInstance`)))
  (`/Engine/EditorBlueprintResources/StandardMacros.IsValid` _savegameobject
    (:`Is Valid`
      (bind _returnvalue (`GameplayStatics.GetCurrentLevelName` true))
      (bind (_value _returnvalue_2) (`BlueprintMapLibrary.Map_Find` (`/Game/SaveSystem/BP_SaveGame.DroppedItemsByLevel` _savegameobject) _returnvalue))
      (if _returnvalue_2
        (for _array_element (`.DroppedItemSnapshots_3_85FD410C43BD3BFB27C697B8A60E77B6` (break `/Game/SaveSystem/S_DroppedItemSnapshotArray` _value))
          (bind (_inventoryitemsnapshot _transform) (break `/Game/SaveSystem/S_DroppedItemSnapshot` _array_element))
          (bind _returnvalue_3 (`|SpawnActorFromClass` "/Game/InventorySystem/BP_PickupItem.BP_PickupItem_C" _transform "Undefined" "MultiplyWithRoot" null _inventoryitemsnapshot null))
          (`KismetArrayLibrary.Array_Add` (`Actor.Tags` _returnvalue_3) "DroppedItem"))))
    (:`Is Not Valid`
      (`KismetSystemLibrary.PrintString` "world persistence component says save game obj not valid"))))

(event `HandleLoadPlayer`
  (params (PlayerController :type "Controller Object Reference"))
  (bind _returnvalue (`Controller.K2_GetPawn` PlayerController))
  (bind _returnvalue_2 (`Actor.GetComponentByClass` _returnvalue "/Game/InventorySystem/BPC_InventoryManager.BPC_InventoryManager_C"))
  (bind _returnvalue_3 (`Actor.GetComponentByClass` _returnvalue "/Game/EquipmentSystem/BPC_EquipmentManager.BPC_EquipmentManager_C"))
  ; Load/save player
  (`/Engine/EditorBlueprintResources/StandardMacros.IsValid` _returnvalue_2
    (:`Is Valid`
      (`/Game/InventorySystem/BPC_InventoryManager.HandleLoadInventory` _returnvalue_2)
      (`/Engine/EditorBlueprintResources/StandardMacros.IsValid` _returnvalue_3
        (:`Is Valid`
          (`/Game/EquipmentSystem/BPC_EquipmentManager.HandleLoadEquipment` _returnvalue_3)
          (bind _asbp_player (cast `/Game/Characters/BP_Player` _returnvalue)
            (:`then`
              (`/Game/Characters/BP_Player.HandleLoadPlayerState` _asbp_player))
            (:`CastFailed`
              (`KismetSystemLibrary.PrintString` "off3"))))
        (:`Is Not Valid`
          (`KismetSystemLibrary.PrintString` "off2"))))
    (:`Is Not Valid`
      (`KismetSystemLibrary.PrintString` "off1"))))

(event `HandleSavePlayer`
  (params (PlayerController :type "Controller Object Reference"))
  (bind _returnvalue (`Controller.K2_GetPawn` PlayerController))
  ; Load/save player
  (`self.HandleSaveLevelState`)
  (`/Game/InventorySystem/BPC_InventoryManager.HandleSaveInventory` (`Actor.GetComponentByClass` _returnvalue "/Game/InventorySystem/BPC_InventoryManager.BPC_InventoryManager_C"))
  (`/Game/EquipmentSystem/BPC_EquipmentManager.HandleSaveEquipment` (`Actor.GetComponentByClass` _returnvalue "/Game/EquipmentSystem/BPC_EquipmentManager.BPC_EquipmentManager_C"))
  (bind _asbp_player (cast `/Game/Characters/BP_Player` _returnvalue)
    (:`then`
      (`/Game/Characters/BP_Player.HandleSavePlayerState` _asbp_player))
    (:`CastFailed`
      _))
  (message `/Game/SaveSystem/BPI_SaveAndLoadManager.SaveGame` (`GameplayStatics.GetGameInstance`)))