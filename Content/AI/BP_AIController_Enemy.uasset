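; Enemy AI controller that starts the enemy behavior tree and reacts to sighting a pawn.
; On BeginPlay it runs BT_Enemy.
; When its PawnSensing component sees a pawn, it flags IsTargetAcquired and stores the pawn as Target in the blackboard.
; It also sets that pawn as CombatTargetActor on the controlled BP_Character_Base, with no filtering of which pawn was seen.
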(event `self.ReceiveBeginPlay`
  (`self.RunBehaviorTree` "/Game/AI/BT_Enemy.BT_Enemy"))

(event `self.PawnSensing.OnSeePawn`
  (params (Pawn :type "Pawn Object Reference"))
  (`BlackboardComponent.SetValueAsBool` (`AIBlueprintHelperLibrary.GetBlackboard` null) "IsTargetAcquired" true)
  (`BlackboardComponent.SetValueAsObject` (`AIBlueprintHelperLibrary.GetBlackboard` null) "Target" Pawn)
  (bind _asbp_character_base (cast `/Game/Characters/BP_Character_Base` (`self.K2_GetPawn`)))
  (set `/Game/Characters/BP_Character_Base.CombatTargetActor` Pawn _asbp_character_base))

(fn `UserConstructionScript`)