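; Base area actor that applies a gameplay effect to overlapping actors with an Ability System Component and removes it when they leave.
; On overlap, it builds a spec from the Effect class with a tag-based SetByCaller magnitude and itself as causer.
; A next-frame pass at BeginPlay also handles actors already inside.
; Exit removes all stacks of that effect class, without filtering by source area.
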(event `self.ReceiveBeginPlay`
  (`KismetSystemLibrary.DelayUntilNextFrame`)
  (for _array_element (`self.GetOverlappingActors` self null)
    (`self.HandleActorBeginOverlap` _array_element)))

(event `self.ReceiveActorBeginOverlap`
  (params (OtherActor :type "Actor Object Reference"))
  (`self.HandleActorBeginOverlap` OtherActor))

(event `self.ReceiveActorEndOverlap`
  (params (OtherActor :type "Actor Object Reference"))
  (`self.HandleActorEndOverlap` OtherActor))

(event `HandleActorBeginOverlap`
  (params (OtherActor :type "Actor Object Reference"))
  (bind _returnvalue (`AbilitySystemBlueprintLibrary.GetAbilitySystemComponent` OtherActor))
  (`/Engine/EditorBlueprintResources/StandardMacros.IsValid` _returnvalue
    (:`Is Valid`
      (bind _returnvalue_2 (`AbilitySystemBlueprintLibrary.MakeSpecHandleByClass` (`self.Effect`) null self))
      (bind _returnvalue_3 (`AbilitySystemBlueprintLibrary.AssignTagSetByCallerMagnitude` _returnvalue_2 (`self.EffectDataTag`) (`self.EffectMagnitude`)))
      (`AbilitySystemComponent.BP_ApplyGameplayEffectSpecToSelf` _returnvalue _returnvalue_3))))

(event `HandleActorEndOverlap`
  (params (OtherActor :type "Actor Object Reference"))
  (bind _returnvalue (`AbilitySystemBlueprintLibrary.GetAbilitySystemComponent` OtherActor))
  (`/Engine/EditorBlueprintResources/StandardMacros.IsValid` _returnvalue
    (:`Is Valid`
      (`AbilitySystemComponent.RemoveActiveGameplayEffectBySourceEffect` _returnvalue (`self.Effect`) null -1))))

(fn `UserConstructionScript`)