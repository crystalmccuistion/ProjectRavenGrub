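; GA_Heal is a gameplay ability that heals the owning avatar and uses up a charge of the Life Gem item.
; It plays a power-up montage while a blocking action message is active, and waits for a gameplay event to commit.
; On that event it applies an instant heal effect with a set-by-caller magnitude, then decrements the gem's limited-use fragment through the inventory manager.
; The ability ends when the montage completes or is interrupted.
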(event `self.K2_ActivateAbility`
  (bind _returnvalue (`self.GetAvatarActorFromActorInfo`))
  (bind _returnvalue_2 (`Actor.GetComponentByClass` (`self.GetAvatarActorFromActorInfo`) "/Game/InventorySystem/BPC_InventoryManager.BPC_InventoryManager_C"))
  (`AbilityTask_PlayMontageAndWait.CreatePlayMontageAndWaitProxy` "None" "/Game/Characters/Animations/Actions/Doll_PowerUp_Montage.Doll_PowerUp_Montage" 1.0 "None" true 1.0 0.0 true
    (:`then`
      (message `/Game/AbilitySystem/BPI_AbilitySystem.StartBlockingAction` (`self.GetAvatarActorFromActorInfo`))
      (`AbilityTask_WaitGameplayEvent.WaitGameplayEvent` (struct :`TagName` "Event") null
        (:`EventReceived`
          (`self.K2_CommitAbility`)
          (bind _returnvalue_3 (`AbilitySystemBlueprintLibrary.MakeSpecHandleByClass` "/Game/AbilitySystem/Effects/GE_Heal_Instant.GE_Heal_Instant_C" _returnvalue _returnvalue))
          (bind _returnvalue_4 (`AbilitySystemBlueprintLibrary.AssignTagSetByCallerMagnitude` _returnvalue_3 (struct :`TagName` "Data.Heal") 50.0))
          (`self.K2_ApplyGameplayEffectSpecToOwner` _returnvalue_4)
          (`/Engine/EditorBlueprintResources/StandardMacros.IsValid` _returnvalue_2
            (:`Is Valid`
              (bind _inventoryitem (`/Game/InventorySystem/BPC_InventoryManager.FindItemByDefinition` _returnvalue_2 "/Game/InventorySystem/Items/Item_LifeGem.Item_LifeGem_C"))
              (bind _iteminstance (break `/Game/InventorySystem/Types/S_InventoryItem` _inventoryitem))
              (`/Engine/EditorBlueprintResources/StandardMacros.IsValid` _iteminstance
                (:`Is Valid`
                  (`/Game/InventorySystem/Fragments/BP_ItemFragment_LimitedUse.DecrementUsesLeft` (`ItemInstance.FindFragmentByClass` _iteminstance "/Game/InventorySystem/Fragments/BP_ItemFragment_LimitedUse.BP_ItemFragment_LimitedUse_C") _iteminstance)
                  (`/Game/InventorySystem/BPC_InventoryManager.OnInventoryChanged` _returnvalue_2))))))))
    (:`OnCompleted`
      (`self.K2_EndAbility` :!label _label))
    (:`OnInterrupted`
      (goto _label))
    (:`OnCancelled`
      (goto _label))))

(event `self.K2_OnEndAbility`
  (params (bWasCancelled :type Boolean))
  (`parent.K2_OnEndAbility` bWasCancelled)
  (message `/Game/AbilitySystem/BPI_AbilitySystem.StopBlockingAction` (`self.GetAvatarActorFromActorInfo`)))