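; Base melee attack ability that plays a montage using the main-hand weapon from the avatar's equipment manager.
; Montage gameplay events open and close the weapon's hit scan, passing a SetByCaller damage effect spec and snapping the character's direction on start.
; At the anim exit point, players end early unless this same ability is queued, while other avatars continue.
; Action blocking starts with the montage; ability end clears it and stops the hit scan.
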(event `self.K2_ActivateAbility`
  (bind _returnvalue (`Actor.GetComponentByClass` (`self.GetAvatarActorFromActorInfo`) "/Game/EquipmentSystem/BPC_EquipmentManager.BPC_EquipmentManager_C"))
  (`/Engine/EditorBlueprintResources/StandardMacros.IsValid` _returnvalue
    (:`Is Valid`
      (bind _output_get (set `self.EquipmentManager` _returnvalue))
      (bind _equipment (`/Game/EquipmentSystem/BPC_EquipmentManager.FindEquipmentInSlot` _output_get (struct :`TagName` "Equipment.Slot.MainHand")))
      (`/Engine/EditorBlueprintResources/StandardMacros.IsValid` _equipment
        (:`Is Valid`
          (bind _asbp_weapon_base (cast `/Game/WeaponSystem/BP_Weapon_Base` (`EquipmentInstance.SpawnedEquipmentActor` _equipment))
            (:`then`
              (set `self.SpawnedWeapon` _asbp_weapon_base)
              (`self.K2_CommitAbility`)
              (bind _montage (`self.Montage`)
                (:`then`
                  (`AbilityTask_PlayMontageAndWait.CreatePlayMontageAndWaitProxy` "None" _montage 1.0 "None" true 1.0 0.0 true
                    (:`then`
                      (`self.OnMontageStart`)
                      (`AbilityTask_WaitGameplayEvent.WaitGameplayEvent` (struct :`TagName` "Event.HitScan.Start") null
                        (:`then`
                          (`AbilityTask_WaitGameplayEvent.WaitGameplayEvent` (struct :`TagName` "Event.HitScan.End") null
                            (:`then`
                              (`AbilityTask_WaitGameplayEvent.WaitGameplayEvent` (struct :`TagName` "Event.AnimExitPoint") null
                                (:`EventReceived`
                                  (if (not (`self.ShouldContinue`))
                                    (`self.K2_EndAbility`)))))
                            (:`EventReceived`
                              (`self.HandleHitScanEnd`))))
                        (:`EventReceived`
                          (`self.HandleHitScanStart`))))
                    (:`OnCompleted`
                      (`self.K2_EndAbility` :!label _label))
                    (:`OnInterrupted`
                      (goto _label))
                    (:`OnCancelled`
                      (goto _label))))
                (:`else`
                  (`self.K2_EndAbility` :!label _label_2))))
            (:`CastFailed`
              (goto _label_2))))
        (:`Is Not Valid`
          (goto _label_2))))
    (:`Is Not Valid`
      (goto _label_2))))

(event `self.K2_OnEndAbility`
  (params (bWasCancelled :type Boolean))
  (bind _spawnedweapon (`self.SpawnedWeapon`))
  (`parent.K2_OnEndAbility` bWasCancelled)
  (message `/Game/AbilitySystem/BPI_AbilitySystem.StopBlockingAction` (`self.GetAvatarActorFromActorInfo`))
  (`/Engine/EditorBlueprintResources/StandardMacros.IsValid` _spawnedweapon
    (:`Is Valid`
      (`/Game/WeaponSystem/BP_Weapon_Base.HitScanEnd` _spawnedweapon))))

(fn `HandleHitScanEnd`
  (bind _spawnedweapon (`self.SpawnedWeapon`)
    (:`then`
      (`/Game/WeaponSystem/BP_Weapon_Base.HitScanEnd` _spawnedweapon))
    (:`else`)))

(fn `HandleHitScanStart`
  (bind _gameplayeffect (`self.GameplayEffect`)
    (:`then`
      (bind _spawnedweapon (`self.SpawnedWeapon`)
        (:`then`
          (bind _returnvalue (`AbilitySystemBlueprintLibrary.AssignTagSetByCallerMagnitude` (`self.MakeOutgoingGameplayEffectSpec` _gameplayeffect) (struct :`TagName` "Data.Damage") (`self.DamageMagnitude`)))
          (`/Game/WeaponSystem/BP_Weapon_Base.HitScanStart` _spawnedweapon _returnvalue)
          (bind _asbp_character_base (cast `/Game/Characters/BP_Character_Base` (`self.GetAvatarActorFromActorInfo`)))
          (`/Game/Characters/BP_Character_Base.HandleSnapDirection` _asbp_character_base))
        (:`else`)))
    (:`else`)))

(fn `OnMontageStart`
  (message `/Game/AbilitySystem/BPI_AbilitySystem.StartBlockingAction` (`self.GetAvatarActorFromActorInfo`)))

(fn `ShouldContinue`
  (returns (Value :type Boolean))
  (bind _asbp_player (cast `/Game/Characters/BP_Player` (`self.GetAvatarActorFromActorInfo`))
    (:`then`
      (return (== (`/Game/Characters/BP_Player.QueuedAbility` _asbp_player) (`GameplayStatics.GetObjectClass` self))))
    (:`CastFailed`
      (return true))))