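; Gameplay ability for equipping a weapon, still unfinished: it only gathers references and performs no equip action.
; When activated from a gameplay event, it finds the avatar's equipment manager component and, if that is valid, its weapon manager, storing both.
; A switch on the event's first target tag is present but unconnected, and the ability never explicitly ends.
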(event `self.K2_ActivateAbilityFromEvent`
  (params (EventData :type "GameplayEventData Structure (by ref)"))
  (bind _returnvalue (`Actor.GetComponentByClass` (`self.GetAvatarActorFromActorInfo`) "/Game/WeaponSystem/BPC_WeaponManager.BPC_WeaponManager_C"))
  (bind _returnvalue_2 (`Actor.GetComponentByClass` (`self.GetAvatarActorFromActorInfo`) "/Game/EquipmentSystem/BPC_EquipmentManager.BPC_EquipmentManager_C"))
  (`/Engine/EditorBlueprintResources/StandardMacros.IsValid` _returnvalue_2
    (:`Is Valid`
      (set `self.EquipmentManager` _returnvalue_2)
      (`/Engine/EditorBlueprintResources/StandardMacros.IsValid` _returnvalue
        (:`Is Valid`
          (set `self.WeaponManager` _returnvalue))))))