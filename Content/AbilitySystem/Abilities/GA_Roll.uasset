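; GA_Roll is a Gameplay Ability for a dodge roll that grants temporary invincibility and requires stamina above zero.
; It snaps the character toward movement input, plays a forward dodge montage, commits, starts action blocking and invincibility, and adds a busy gameplay cue.
; Montage notifies end invincibility and the ability, and ending the ability releases the block.
; Avatar state changes go through message calls.
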(event `self.K2_ActivateAbility`
  (bind _asbp_character_base (cast `/Game/Characters/BP_Character_Base` (`self.GetAvatarActorFromActorInfo`))
    (:`then`
      (`/Game/Characters/BP_Character_Base.SnapDirectionToMovementInput` _asbp_character_base))
    (:`CastFailed`
      _))
  (bind _notifyname (`|PlayMontage` (`self.GetOwningComponentFromActorInfo`) "/Game/Characters/Animations/Roll/Dodge_F_Montage_ChaserDoll.Dodge_F_Montage_ChaserDoll")
    (:`then`
      (`self.K2_CommitAbility`)
      (message `/Game/AbilitySystem/BPI_AbilitySystem.StartBlockingAction` (`self.GetAvatarActorFromActorInfo`))
      (message `/Game/Blueprints/BPI_Combat.BeginInvincibility` (`self.GetAvatarActorFromActorInfo`))
      (`self.K2_AddGameplayCue` (struct :`TagName` "GameplayCue.Busy.Roll")))
    (:`OnNotifyBegin`
      (if (== _notifyname "EndInvincibility")
        (message `/Game/Blueprints/BPI_Combat.EndInvincibility` (`self.GetAvatarActorFromActorInfo`))
        (elif (== _notifyname "StopBlockingAction")
          (`self.K2_EndAbility`))))))

(event `self.K2_OnEndAbility`
  (params (bWasCancelled :type Boolean))
  (message `/Game/AbilitySystem/BPI_AbilitySystem.StopBlockingAction` (`self.GetAvatarActorFromActorInfo`))
  (`parent.K2_OnEndAbility` bWasCancelled))

(fn `K2_CanActivateAbility`
  (params (ActorInfo :type "GameplayAbilityActorInfo Structure") (Handle :type "GameplayAbilitySpecHandle Structure"))
  (returns (RelevantTags :type "GameplayTagContainer Structure") (ReturnValue :type Boolean))
  (bind _ascharacter_base (cast `CharacterBase` (`self.GetAvatarActorFromActorInfo`))
    (:`then`
      (bind (_ascstamina_basevalue _ascstamina_currentvalue) (break `GameplayAttributeData` (`BasicAttributeSet.AscStamina` (`CharacterBase.BasicAttributeSet` _ascharacter_base))))
      (return (struct) (> _ascstamina_currentvalue 0.0)))
    (:`CastFailed`
      (return (struct) true))))