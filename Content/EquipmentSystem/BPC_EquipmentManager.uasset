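; Actor component that manages a character's equipped items, toggling equip state and replacing whatever occupies the same slot.
; Equipping builds an EquipmentInstance from the item's Equippable fragment, grants the spawned weapon's abilities and sends an equip gameplay event.
; Granted ability tags are mapped by slot for removal on unequip.
; Equipment saves as inventory indices through the game instance's save object and reloads by re-equipping silently.
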(event `self.ReceiveBeginPlay`
  (bind _returnvalue (`self.GetOwner`))
  (set `self.InventoryManager` (`Actor.GetComponentByClass` _returnvalue "/Game/InventorySystem/BPC_InventoryManager.BPC_InventoryManager_C"))
  (bind _asbp_character_base (cast `/Game/Characters/BP_Character_Base` _returnvalue))
  (set `self.OwningCharacter` _asbp_character_base))

(fn `EquipItem`
  (params (ItemInstance :type "ItemInstance Object Reference") (SuppressSound :type Boolean :default true))
  (bind _equipmentinstance (`self.FindEquipmentByItemInstance` ItemInstance))
  (bind _equipmentslotabilitytagsmap_equipmentabilitiesmap (break `/Game/EquipmentSystem/S_EquipmentSlotAbilityTagsMap` (`self.EquipmentSlotAbilityTagsMap`)))
  (bind _equipment (`self.FindEquipmentInSlot` (defaults `Object` (`InventoryFragment_Equippable.EquipmentDefinition` (`ItemInstance.FindFragmentByClass` (`local.ItemInstance`) "/Script/ProjectRavenGrub.InventoryFragment_Equippable")))))
  ; If item already equipped, unequip it
  (`/Engine/EditorBlueprintResources/StandardMacros.IsValid` _equipmentinstance
    (:`Is Valid`
      (`self.UnequipItem` _equipmentinstance)
      (`self.OnEquipmentChanged`)
      (if (not (`local.SuppressSound`))
        (`GameplayStatics.PlaySoundAtLocation` (`self.UnequipSound`) (`Actor.K2_GetActorLocation` (`self.GetOwner`)) (struct) 1.0 1.0 0.0 null null null null)))
    (:`Is Not Valid`
      ; If slot already occupied, unequip existing slot item
      (`/Engine/EditorBlueprintResources/StandardMacros.IsValid` _equipment
        (:`Is Valid`
          (`self.UnequipItem` _equipment))
        (:`Is Not Valid`
          _))
      ; Equip item
      (bind _returnvalue (`|GenericCreateObject` "/Script/ProjectRavenGrub.EquipmentInstance"))
      (`EquipmentInstance.Initialize` _returnvalue (`local.ItemInstance`) (`self.OwningCharacter`))
      (`KismetArrayLibrary.Array_AddUnique` (`self.EquippedItems`) _returnvalue)
      (bind _returnvalue_2 (`CharacterBase.GrantAbilities` (`self.OwningCharacter`) (`self.GetWeaponInfo` _returnvalue)))
      (`BlueprintMapLibrary.Map_Add` _equipmentslotabilitytagsmap_equipmentabilitiesmap (defaults `Object` (`InventoryFragment_Equippable.EquipmentDefinition` (`ItemInstance.FindFragmentByClass` (`local.ItemInstance`) "/Script/ProjectRavenGrub.InventoryFragment_Equippable"))) (make `/Game/EquipmentSystem/S_AbilityTags` _returnvalue_2))
      (`AbilitySystemBlueprintLibrary.SendGameplayEventToActor` (`self.OwningCharacter`) (struct :`TagName` "Event.Weapon.Equip") (make `GameplayEventData` (struct) null null null null (struct) (struct) (`BlueprintGameplayTagLibrary.MakeGameplayTagContainerFromTag` (`.SlotTag` (defaults `Object` (`EquipmentInstance.EquipmentDefinition` _returnvalue))))))
      (`self.OnEquipmentChanged`)
      (if (not (`local.SuppressSound`))
        (`GameplayStatics.PlaySoundAtLocation` (`self.EquipSound`) (`Actor.K2_GetActorLocation` (`self.GetOwner`)) (struct) 1.0 1.0 0.0 null null null null)))))

(fn `FindEquipmentByItemInstance`
  (params (ItemInstance :type "ItemInstance Object Reference"))
  (returns (EquipmentInstance :type "EquipmentInstance Object Reference"))
  (for _array_element (`self.EquippedItems`)
    (if (== (`EquipmentInstance.SourceItemInstance` _array_element) ItemInstance)
      (return _array_element)))
  (return null))

(fn `FindEquipmentInSlot`
  (params (SlotTag :type "GameplayTag Structure"))
  (returns (Equipment :type "EquipmentInstance Object Reference"))
  (for _array_element (`self.EquippedItems`)
    (if (== (defaults `Object` (`EquipmentInstance.EquipmentDefinition` _array_element)) SlotTag)
      (return _array_element)))
  (return null))

(fn `GetWeaponInfo`
  (params (EquipmentInstance :type "EquipmentInstance Object Reference"))
  (returns (AbilitiesToGrant :type "Array of GameplayAbility Class Reference") (AnimClass :type "AnimInstance Class Reference"))
  (`/Engine/EditorBlueprintResources/StandardMacros.IsValid` EquipmentInstance
    (:`Is Valid`
      (bind _spawnedequipmentactor (`EquipmentInstance.SpawnedEquipmentActor` EquipmentInstance)
        (:`then`
          (bind _asbp_weapon_base (cast `/Game/WeaponSystem/BP_Weapon_Base` _spawnedequipmentactor)
            (:`then`
              (bind (_abilitiestogrant _animclass) (break `/Game/WeaponSystem/S_WeaponInfo` (`/Game/WeaponSystem/BP_Weapon_Base.WeaponInfo` _asbp_weapon_base)))
              (return _abilitiestogrant _animclass))
            (:`CastFailed`
              _)))
        (:`else`
          _)))
    (:`Is Not Valid`
      _))
  (return (`|MakeArray` null :!type "GameplayAbility Class Reference") "/Game/Characters/Animations/ABP_Doll_Unarmed.ABP_Doll_Unarmed_C"))

(fn `HandleLoadEquipment`
  (bind _savegameobject (message `/Game/SaveSystem/BPI_SaveAndLoadManager.GetSaveGameObject` (`GameplayStatics.GetGameInstance`)))
  (`/Engine/EditorBlueprintResources/StandardMacros.IsValid` _savegameobject
    (:`Is Valid`
      (for _array_element (`/Game/SaveSystem/BP_SaveGame.EquippedItemIndices` _savegameobject)
        (bind _output_iteminstance (break `/Game/InventorySystem/Types/S_InventoryItem` (`|GetArrayItem` (`/Game/InventorySystem/BPC_InventoryManager.InventoryItems` (`self.InventoryManager`)) _array_element)))
        (`self.EquipItem` _output_iteminstance)))))

(fn `HandleSaveEquipment`
  (bind _savegameobject (message `/Game/SaveSystem/BPI_SaveAndLoadManager.GetSaveGameObject` (`GameplayStatics.GetGameInstance`)))
  (`/Engine/EditorBlueprintResources/StandardMacros.IsValid` _savegameobject
    (:`Is Valid`
      (bind _equippeditemindices (`/Game/SaveSystem/BP_SaveGame.EquippedItemIndices` _savegameobject))
      (`KismetArrayLibrary.Array_Clear` _equippeditemindices)
      (for _array_element (`self.EquippedItems`)
        (bind _item_index (`/Game/InventorySystem/BPC_InventoryManager.FindItemByInstance` (`self.InventoryManager`) (`EquipmentInstance.SourceItemInstance` _array_element)))
        (if (> _item_index -1)
          (`KismetArrayLibrary.Array_Add` _equippeditemindices _item_index))))))

(fn `UnequipItem`
  (params (EquipmentInstance :type "EquipmentInstance Object Reference"))
  (bind _equipmentslotabilitytagsmap_equipmentabilitiesmap (break `/Game/EquipmentSystem/S_EquipmentSlotAbilityTagsMap` (`self.EquipmentSlotAbilityTagsMap`)))
  (bind (_value _returnvalue) (`BlueprintMapLibrary.Map_Find` _equipmentslotabilitytagsmap_equipmentabilitiesmap (`.SlotTag` (defaults `Object` (`EquipmentInstance.EquipmentDefinition` EquipmentInstance)))))
  (`EquipmentInstance.HandleUnequipItem` EquipmentInstance (`self.OwningCharacter`))
  (if _returnvalue
    (`CharacterBase.RemoveAbilities` (`self.OwningCharacter`) (`.AbilityTags_4_EA261153401C243C8EB082961901D2A0` (break `/Game/EquipmentSystem/S_AbilityTags` _value))))
  (`KismetArrayLibrary.Array_RemoveItem` (`self.EquippedItems`) EquipmentInstance))