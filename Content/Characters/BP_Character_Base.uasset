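; Base character Blueprint providing shared combat, damage and interaction behavior, with health queries and damage handling delegated to DamageSystem.
; GAS async listeners end stamina regen at max, restart a timer on poise changes and trigger death on Status.Dead.
; Death ragdolls the mesh with an impulse, fires a death dispatcher and removes the interaction radius.
; Helper functions toggle strafing from running and camera-lock tags, snap or face toward targets, and read starting-sword attack power.
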(event `self.ReceiveBeginPlay`
  (bind (_asynctaskproxy _attribute _newvalue _oldvalue) (`AbilityAsync_WaitAttributeChanged.WaitForAttributeChanged` null (struct :`AttributeName` "AscStamina" :`Attribute` "/Script/ProjectRavenGrub.BasicAttributeSet:AscStamina" :`AttributeOwner` "/Script/CoreUObject.Class'/Script/ProjectRavenGrub.BasicAttributeSet'"))
    (:`then`
      (`AbilityAsync_WaitAttributeChanged.WaitForAttributeChanged` null (struct :`AttributeName` "AscPoise" :`Attribute` "/Script/ProjectRavenGrub.BasicAttributeSet:AscPoise" :`AttributeOwner` "/Script/CoreUObject.Class'/Script/ProjectRavenGrub.BasicAttributeSet'")
        (:`then`
          (`AbilityAsync_WaitGameplayTagAdded.WaitGameplayTagAddToActor` null (struct :`TagName` "Status.Dead")
            (:`Added`
              (`self.RespondToDeath`))))
        (:`Changed`
          (`self.HandlePoiseChanged`))))
    (:`Changed`
      (`self.HandleStaminaChanged` _newvalue _oldvalue))))

(event `HandleStaminaChanged`
  (params (NewValue :type "Float (double-precision)") (OldValue :type "Float (double-precision)"))
  (bind (_ascmaxstamina_basevalue _ascmaxstamina_currentvalue) (break `GameplayAttributeData` (`BasicAttributeSet.AscMaxStamina` (`self.BasicAttributeSet`))))
  (if (== NewValue _ascmaxstamina_currentvalue)
    (`AbilitySystemComponent.RemoveActiveEffectsWithGrantedTags` (`self.AbilitySystemComponent`) (struct :`GameplayTags` (struct :`(TagName` "Status.Stamina.Regen"))))))

(event `/Game/Blueprints/BPI_Interactable.Interact`
  (params (Interactor :type "Actor Object Reference"))
  ; On Interacted
  (if (not (`DamageSystemComponent.GetIsDead` (`self.DamageSystem`)))
    (`self.RespondToInteract`)))

(event `RespondToInteract`
  (bind _interactableradius (`self.InteractableRadius`))
  ; On Interacted
  (`/Engine/EditorBlueprintResources/StandardMacros.IsValid` _interactableradius
    (:`Is Valid`
      (`GameplayStatics.PlaySoundAtLocation` "/Game/UI/Sound/UI_Select_Cue.UI_Select_Cue" (`SceneComponent.K2_GetComponentLocation` _interactableradius) (struct) 1.0 1.0 0.0 null null null null))))

(event `RespondToDeath`
  (bind _mesh (`self.Mesh`))
  (`KismetSystemLibrary.PrintString` "BP_Character_Base says RespondToDeath")
  (`PrimitiveComponent.SetCollisionEnabled` (`self.CapsuleComponent`) "NoCollision")
  (`PrimitiveComponent.SetSimulatePhysics` _mesh true)
  (`PrimitiveComponent.SetCollisionEnabled` _mesh "QueryAndPhysics")
  (`CharacterMovementComponent.DisableMovement` (`self.CharacterMovement`))
  (`PrimitiveComponent.AddImpulseAtLocation` _mesh (`KismetMathLibrary.MakeVector` (.x (* (`self.GetActorForwardVector` self) (`KismetMathLibrary.Conv_DoubleToVector` -10000.0))) (.y (* (`self.GetActorForwardVector` self) (`KismetMathLibrary.Conv_DoubleToVector` -10000.0))) -15000.0) (`self.K2_GetActorLocation` self) "None")
  (`self.DeathEventDispatcher`)
  (`ActorComponent.K2_DestroyComponent` (`self.InteractableRadius`))
  (`GameplayStatics.PlaySoundAtLocation` "/Game/Sounds/SFX_KillEnemy_Cue.SFX_KillEnemy_Cue" (`self.K2_GetActorLocation` self) (struct) 1.0 1.0 0.0 null null null null))

(fn `FaceTarget`
  (params (TargetActor :type "Actor Object Reference"))
  (`Controller.SetControlRotation` (`self.GetController`) (`KismetMathLibrary.FindLookAtRotation` (`self.K2_GetActorLocation` self) (`self.K2_GetActorLocation` TargetActor))))

(fn `GetAttributeManager`
  (returns (BPC_AttributeManager :type "/Game/Blueprints/BPC_AttributeManager Object Reference"))
  (return (`self.BPC_AttributeManager`)))

(fn `GetCurrentHealth`
  (returns (ReturnValue :type "Float (single-precision)"))
  (return (`DamageSystemComponent.GetCurrentHealth` (`self.DamageSystem`))))

(fn `GetInteractPrompt`
  (returns (PromptText :type Text))
  (return "Talk"))

(fn `GetInteractSocket`
  (returns (InteractSocket :type "SceneComponent Object Reference"))
  (return (`self.InteractSocket`)))

(fn `GetIsDead`
  (returns (ReturnValue :type Boolean))
  (return (`DamageSystemComponent.GetIsDead` (`self.DamageSystem`))))

(fn `GetMaxHealth`
  (returns (ReturnValue :type "Float (single-precision)"))
  (return (`DamageSystemComponent.GetMaxHealth` (`self.DamageSystem`))))

(fn `GetMoveDirectionKey`
  (returns (MoveDirectionKey :type "Key Structure"))
  (for _array_element (`EnhancedInputSubsystemInterface.QueryKeysMappedToAction` (pcsubsystem `EnhancedInputLocalPlayerSubsystem` (`GameplayStatics.GetPlayerController` 0)) "/Game/Input/Actions/IA_Move.IA_Move")
    (if (`PlayerController.IsInputKeyDown` (`GameplayStatics.GetPlayerController` 0) _array_element)
      (return _array_element))))

(fn `GetWeaponAttackPower`
  (returns (`Attack Power` :type "Float (single-precision)"))
  (for _array_element (`/Game/EquipmentSystem/BPC_EquipmentManager.EquippedItems` (`self.BPC_EquipmentManager`))
    (bind _sourceiteminstance (`EquipmentInstance.SourceItemInstance` _array_element))
    (if (== (`ItemInstance.ItemDefinition` _sourceiteminstance) "/Game/InventorySystem/Items/Item_Equipment_StartingSword.Item_Equipment_StartingSword_C")
      (return (`ItemInstance.GetStatValue` _sourceiteminstance (struct :`TagName` "Item.Stat.AttackPower")))
      (else
        (return 0.0)))))

(fn `HandlePoiseChanged`
  (`KismetSystemLibrary.K2_ClearAndInvalidateTimerHandle` (`self.PoiseRegenTimer`))
  (bind _returnvalue (`KismetSystemLibrary.K2_SetTimerDelegate` :`Time` (`self.PoiseRegenTimerDuration`)))
  (set `self.PoiseRegenTimer` _returnvalue))

(fn `HandleSnapDirection`
  (`self.SnapDirectionToTarget` (`self.CombatTargetActor`)))

(fn `InitializeInventory`)

(fn `SnapDirectionToMovementInput`
  (returns (Success :type Boolean))
  (bind _returnvalue (`self.GetLastMovementInputVector`))
  (if (not (`KismetMathLibrary.Vector_IsZero` _returnvalue))
    (`self.K2_SetActorRotation` (`KismetMathLibrary.Conv_VectorToRotator` _returnvalue))
    (return true)
    (else
      (return false))))

(fn `SnapDirectionToTarget`
  (params (DirectionTarget :type "Actor Object Reference"))
  (bind (_returnvalue_roll _returnvalue_pitch _returnvalue_yaw) (`KismetMathLibrary.BreakRotator` (`KismetMathLibrary.FindLookAtRotation` (`self.K2_GetActorLocation` self) (`self.K2_GetActorLocation` (`local.DirectionTarget`)))))
  (`/Engine/EditorBlueprintResources/StandardMacros.IsValid` DirectionTarget
    (:`Is Valid`
      (`self.K2_SetActorRotation` self (`KismetMathLibrary.MakeRotator` _returnvalue_roll _returnvalue_pitch _returnvalue_yaw) false))))

(fn `StartStrafing`
  (bind _charactermovement (`self.CharacterMovement`))
  (set `CharacterMovementComponent.bOrientRotationToMovement` false _charactermovement)
  (set `CharacterMovementComponent.bUseControllerDesiredRotation` true _charactermovement))

(fn `StopStrafing`
  (bind _charactermovement (`self.CharacterMovement`))
  (set `CharacterMovementComponent.bOrientRotationToMovement` true _charactermovement)
  (set `CharacterMovementComponent.bUseControllerDesiredRotation` false _charactermovement))

(fn `TakeDamage`
  (params (DamageInfo :type "DamageInfo Structure (by ref)"))
  (returns (ReturnValue :type Boolean))
  (bind _returnvalue (`DamageSystemComponent.HandleIncomingDamage` (`self.DamageSystem`) DamageInfo))
  (return _returnvalue))

(fn `UpdateStrafing`
  (if (`BlueprintGameplayTagLibrary.HasTag` (`/Game/Blueprints/BPC_TagManager.TagContainer` (`self.BPC_TagManager`)) (struct :`TagName` "Status.Busy.Running"))
    (`self.StopStrafing`)
    (elif (`BlueprintGameplayTagLibrary.HasTag` (`/Game/Blueprints/BPC_TagManager.TagContainer` (`self.BPC_TagManager`)) (struct :`TagName` "Status.CameraLocked"))
      (`self.StartStrafing`)
      (else
        (`self.StopStrafing`)))))

(fn `UserConstructionScript`)