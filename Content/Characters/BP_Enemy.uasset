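; Enemy character Blueprint that extends a parent class with a starting sword, a health bar and a sword-combo light attack.
; On BeginPlay it hides SMRWeapon, adds and uses the sword through the inventory manager, and caches health from the Ability System.
; An attribute-change listener pushes new health values to the vitals widget, which is hidden on death.
; Helpers play the attack montage and return player distance, with a large fallback value.
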(event `self.ReceiveBeginPlay`
  (bind _returnvalue (`AbilitySystemBlueprintLibrary.GetAbilitySystemComponent` null))
  (`parent.ReceiveBeginPlay`)
  (`SceneComponent.SetHiddenInGame` (`self.SM_R_Weapon`) true false)
  (`self.InitializeInventory`)
  (set `self.Health` (`.ReturnValue` (`AbilitySystemBlueprintLibrary.GetFloatAttributeFromAbilitySystemComponent` _returnvalue (struct :`AttributeName` "AscHealth" :`Attribute` "/Script/ProjectRavenGrub.BasicAttributeSet:AscHealth" :`AttributeOwner` "/Script/CoreUObject.Class'/Script/ProjectRavenGrub.BasicAttributeSet'"))))
  (set `self.MaxHealth` (`.ReturnValue` (`AbilitySystemBlueprintLibrary.GetFloatAttributeFromAbilitySystemComponent` _returnvalue (struct :`AttributeName` "AscMaxHealth" :`Attribute` "/Script/ProjectRavenGrub.BasicAttributeSet:AscMaxHealth" :`AttributeOwner` "/Script/CoreUObject.Class'/Script/ProjectRavenGrub.BasicAttributeSet'"))))
  (bind (_asynctaskproxy _attribute _newvalue) (`AbilityAsync_WaitAttributeChanged.WaitForAttributeChanged` null (struct :`AttributeName` "AscHealth" :`Attribute` "/Script/ProjectRavenGrub.BasicAttributeSet:AscHealth" :`AttributeOwner` "/Script/CoreUObject.Class'/Script/ProjectRavenGrub.BasicAttributeSet'"))
    (:`Changed`
      (`self.UpdateEnemyVitalsWidget` _newvalue))))

(event `self.RespondToDamage`
  (params (DamageInfo :type "DamageInfo Structure (by ref)"))
  (`parent.RespondToDamage` DamageInfo))

(event `self.RespondToDeath`
  (`parent.RespondToDeath`)
  (`SceneComponent.SetVisibility` (`self.VitalsWidget`) false false))

(fn `GetDistanceToPlayer`
  (returns (Distance :type "Float (double-precision)"))
  (bind _returnvalue (`GameplayStatics.GetPlayerPawn` 0))
  (`/Engine/EditorBlueprintResources/StandardMacros.IsValid` _returnvalue
    (:`Is Valid`
      (return (`KismetMathLibrary.Vector_Distance` (`self.K2_GetActorLocation` self) (`self.K2_GetActorLocation` _returnvalue))))
    (:`Is Not Valid`
      (return 10000.0))))

(fn `InitializeInventory`
  (`/Game/InventorySystem/BPC_InventoryManager.AddItem` (`self.BPC_InventoryManager`) (make `/Game/InventorySystem/Types/S_InventoryItemSnapshot` "/Game/InventorySystem/Items/Item_Equipment_StartingSword.Item_Equipment_StartingSword_C"))
  (for _array_element (`/Game/InventorySystem/BPC_InventoryManager.InventoryItems` (`self.BPC_InventoryManager`))
    (`/Engine/EditorBlueprintResources/StandardMacros.IsValid` (break `/Game/InventorySystem/Types/S_InventoryItem` _array_element)
      (:`Is Valid`
        (if (== (`ItemInstance.ItemDefinition` (break `/Game/InventorySystem/Types/S_InventoryItem` _array_element)) "/Game/InventorySystem/Items/Item_Equipment_StartingSword.Item_Equipment_StartingSword_C")
          (`/Game/InventorySystem/BPC_InventoryManager.UseItem` (`self.BPC_InventoryManager`) true (break `/Game/InventorySystem/Types/S_InventoryItem` _array_element))
          (return))))))

(fn `LightAttack`
  (returns (`Animation Duration` :type "Float (double-precision)"))
  (bind _returnvalue (`self.PlayAnimMontage` "/Game/Characters/Animations/Attacks/Doll_Attack_SwordCombo_Montage.Doll_Attack_SwordCombo_Montage"))
  (return _returnvalue))

(fn `UpdateEnemyVitalsWidget`
  (params (CurrentHealth :type "Float (double-precision)"))
  (bind _returnvalue (`WidgetComponent.GetWidget` (`self.VitalsWidget`)))
  (`/Engine/EditorBlueprintResources/StandardMacros.IsValid` _returnvalue
    (:`Is Valid`
      (bind _aspopup_enemy_health_bar (cast `/Game/UI/Widgets/Popups/Popup_EnemyHealthBar` _returnvalue))
      (`/Game/UI/Widgets/Popups/Popup_EnemyHealthBar.UpdateHealthPercent` _aspopup_enemy_health_bar CurrentHealth (`self.MaxHealth`)))))

(fn `UserConstructionScript`
  (`parent.UserConstructionScript`))