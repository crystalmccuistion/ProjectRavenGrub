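; Inventory item fragment that gives an item a limited number of uses.
; On instance creation it writes MaxNumberOfUses into the instance's Item.Stat.UsesLeft gameplay-tag stat, so the count lives on each item instance rather than the fragment.
; DecrementUsesLeft lowers that stat by one, clamped between zero and the maximum, and HasUsesLeft reports whether a valid instance has any left.
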(event `self.OnInstanceCreated`
  (params (ItemInstance :type "ItemInstance Object Reference"))
  (`ItemInstance.SetStatValue` ItemInstance (struct :`TagName` "Item.Stat.UsesLeft") (`KismetMathLibrary.Conv_IntToDouble` (`self.MaxNumberOfUses`))))

(fn `DecrementUsesLeft`
  (params (ItemInstance :type "ItemInstance Object Reference"))
  (`ItemInstance.SetStatValue` ItemInstance (struct :`TagName` "Item.Stat.UsesLeft") (`KismetMathLibrary.FClamp` (- (`ItemInstance.GetStatValue` ItemInstance (struct :`TagName` "Item.Stat.UsesLeft")) 1.0) 0.0 (`KismetMathLibrary.Conv_IntToDouble` (`self.MaxNumberOfUses`)))))

(fn `HasUsesLeft`
  (params (ItemInstance :type "ItemInstance Object Reference"))
  (returns (ReturnValue :type Boolean))
  (`/Engine/EditorBlueprintResources/StandardMacros.IsValid` ItemInstance
    (:`Is Valid`
      (if (> (`ItemInstance.GetStatValue` ItemInstance (struct :`TagName` "Item.Stat.UsesLeft")) 0.0)
        (return true)
        (else
          _)))
    (:`Is Not Valid`
      _))
  (return false))