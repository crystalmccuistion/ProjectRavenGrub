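; Inventory component that holds its owner's items as stacks of ItemInstance objects with counts, handling add, use, drop, lookup and save/load.
; AddItem tops up a partial stack through recursive FillAllPartialStacks or creates new instances capped at max stack size.
; Item fragments govern use, consumption and droppability; drops unequip through BPC_EquipmentManager and spawn a BP_PickupItem.
; Snapshots of definition, count and stats carry items into pickups and the save game.
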(event `self.ReceiveBeginPlay`
  (bind _returnvalue (`Actor.GetComponentByClass` (`self.GetOwner`) "/Game/EquipmentSystem/BPC_EquipmentManager.BPC_EquipmentManager_C"))
  (`/Engine/EditorBlueprintResources/StandardMacros.IsValid` _returnvalue
    (:`Is Valid`
      (set `self.EquipmentManager` _returnvalue))))

(fn `AddItem`
  (params (InventoryItemInfo :type "/Game/InventorySystem/Types/S_InventoryItemSnapshot Structure"))
  (locals (RemainingItemCountToAdd :type Integer :default 0))
  (bind (_inventoryiteminfo_itemdefinition _inventoryiteminfo_count _inventoryiteminfo_statsmap) (break `/Game/InventorySystem/Types/S_InventoryItemSnapshot` (`local.InventoryItemInfo`)))
  (bind _returnvalue (`KismetMathLibrary.Min` (`local.RemainingItemCountToAdd`) (`/Game/InventorySystem/BFL_InventoryHelpers.GetItemMaxStackCount` _inventoryiteminfo_itemdefinition)))
  (bind _remainder (`self.FillAllPartialStacks` InventoryItemInfo_ItemDefinition_2_A3779B1A43D0545C699530B85B8CDC87 InventoryItemInfo_Count_5_6884BF844EED2CCBF65EA3B8713B2D3C))
  (bind _output_get (set `local.RemainingItemCountToAdd` _remainder))
  (while (> _output_get 0)
    (bind _returnvalue_2 (`|GenericCreateObject` "/Script/ProjectRavenGrub.ItemInstance"))
    (`ItemInstance.Initialize` _returnvalue_2 _inventoryiteminfo_itemdefinition _inventoryiteminfo_statsmap)
    (`KismetArrayLibrary.Array_Add` (`self.InventoryItems`) (make `/Game/InventorySystem/Types/S_InventoryItem` _returnvalue_2 _returnvalue))
    (set `local.RemainingItemCountToAdd` (- (`local.RemainingItemCountToAdd`) _returnvalue)))
  (`self.OnInventoryChanged`))

(fn `CanDropItem`
  (params (ItemInstance :type "ItemInstance Object Reference"))
  (returns (ReturnValue :type Boolean))
  (bind _returnvalue (`ItemInstance.FindFragmentByClass` (`local.ItemInstance`) "/Script/ProjectRavenGrub.InventoryItemFragment_WorldRepresentation"))
  (if (`KismetArrayLibrary.Array_IsValidIndex` (`self.InventoryItems`) (`self.FindItemByInstance` ItemInstance))
    (`/Engine/EditorBlueprintResources/StandardMacros.IsValid` _returnvalue
      (:`Is Valid`
        (if (`InventoryItemFragment_WorldRepresentation.bCanBeDropped` _returnvalue)
          (return true)
          (else
            _)))
      (:`Is Not Valid`
        _)))
  (return false))

(fn `ConsumeItem`
  (params (ItemInstance :type "ItemInstance Object Reference"))
  (bind _item_index (`self.FindItemByInstance` ItemInstance))
  (bind _output (`|GetArrayItem` (`self.InventoryItems`) _item_index))
  (bind (_iteminstance _count) (break `/Game/InventorySystem/Types/S_InventoryItem` _output))
  (if (<= _count 1)
    ; Use last one, remove item
    (`KismetArrayLibrary.Array_Remove` (`self.InventoryItems`) _item_index)
    (else
      ; New count
      (setmembers `/Game/InventorySystem/Types/S_InventoryItem` :`StructRef` _output :`Count` (- _count 1)))))

(fn `DropItem`
  (params (ItemInstance :type "ItemInstance Object Reference"))
  (returns (Success :type Boolean))
  (if (`self.CanDropItem` ItemInstance)
    (if (`self.IsItemEquipped` ItemInstance)
      (`/Game/EquipmentSystem/BPC_EquipmentManager.UnequipItem` (`self.EquipmentManager`) (`/Game/EquipmentSystem/BPC_EquipmentManager.FindEquipmentByItemInstance` (`self.EquipmentManager`) ItemInstance)))
    (bind _returnvalue (`|SpawnActorFromClass` "/Game/Blueprints/LevelActors/BP_PickupItem.BP_PickupItem_C" (`KismetMathLibrary.MakeTransform` (`self.GetDropLocation`)) "Undefined" "MultiplyWithRoot" null (make `/Game/InventorySystem/Types/S_InventoryItemSnapshot` (`ItemInstance.ItemDefinition` ItemInstance) (`.Count_5_DE33369B4029D74F29A5D9B9116881FD` (break `/Game/InventorySystem/Types/S_InventoryItem` (`.Inventory Item` (`self.FindItemByInstance` ItemInstance)))) (`ItemInstance.StatsMap` ItemInstance)) null))
    (`KismetArrayLibrary.Array_Add` (`Actor.Tags` _returnvalue) "DroppedItem")
    (`KismetArrayLibrary.Array_Remove` (`self.InventoryItems`) (`self.FindItemByInstance` (`local.ItemInstance`)))
    (`self.OnInventoryChanged`)
    (return true)))

(fn `FillAllPartialStacks`
  (params (ItemDefinition :type "ItemDefinition Class Reference") (TotalAmount :type Integer))
  (returns (Remainder :type Integer))
  (locals (AmountAdded :type Integer :default 0))
  (bind (_itemindex _isfound) (`self.FindPartialStack` ItemDefinition))
  (bind _output (`|GetArrayItem` (`self.InventoryItems`) _itemindex))
  (bind (_iteminstance _count) (break `/Game/InventorySystem/Types/S_InventoryItem` _output))
  (if (> TotalAmount 0)
    (if _isfound
      (bind _output_get (set `local.AmountAdded` (`KismetMathLibrary.Min` (- (`/Game/InventorySystem/BFL_InventoryHelpers.GetItemMaxStackCount` (`ItemInstance.ItemDefinition` _iteminstance)) _count) (`local.TotalAmount`))))
      (setmembers `/Game/InventorySystem/Types/S_InventoryItem` :`StructRef` _output :`Count` (+ _output_get _count))
      (bind _remainder (`self.FillAllPartialStacks` (`local.ItemDefinition`) (- (`local.AmountAdded`) (`local.TotalAmount`))))
      (return _remainder)
      (else
        (return TotalAmount)))
    (else
      (return 0))))

(fn `FindAllItems`
  (params (ItemDefinition :type "ItemDefinition Class Reference"))
  (returns (InventoryItems :type "Array of /Game/InventorySystem/Types/S_InventoryItem Structure"))
  (locals (MatchingItems :type "Array of /Game/InventorySystem/Types/S_InventoryItem Structure"))
  (for _array_element (`self.InventoryItems`)
    (if (== (`ItemInstance.ItemDefinition` (`.ItemInstance_7_EF089A1F46A4335E27C140B17A59DF67` (break `/Game/InventorySystem/Types/S_InventoryItem` _array_element))) ItemDefinition)
      (`KismetArrayLibrary.Array_Add` (`local.MatchingItems`) _array_element)))
  (return (`local.MatchingItems`)))

(fn `FindAllItemsOfType`
  (params (ItemType :type "GameplayTag Structure"))
  (returns (FoundItems :type "Array of /Game/InventorySystem/Types/S_InventoryItem Structure"))
  (locals (MatchedItems :type "Array of /Game/InventorySystem/Types/S_InventoryItem Structure"))
  (for _array_element (`self.InventoryItems`)
    (if (`BlueprintGameplayTagLibrary.HasTag` (defaults `Object` (`ItemInstance.ItemDefinition` (`.ItemInstance_7_EF089A1F46A4335E27C140B17A59DF67` (break `/Game/InventorySystem/Types/S_InventoryItem` _array_element)))) ItemType true)
      (`KismetArrayLibrary.Array_AddUnique` (`local.MatchedItems`) _array_element)))
  (return (`local.MatchedItems`)))

(fn `FindItemByDefinition`
  (params (ItemDefinition :type "ItemDefinition Class Reference"))
  (returns (InventoryItem :type "/Game/InventorySystem/Types/S_InventoryItem Structure"))
  (for _array_element (`self.InventoryItems`)
    (if (== (`ItemInstance.ItemDefinition` (`.ItemInstance_7_EF089A1F46A4335E27C140B17A59DF67` (break `/Game/InventorySystem/Types/S_InventoryItem` _array_element))) ItemDefinition)
      (return _array_element)))
  (return))

(fn `FindItemByInstance`
  (params (ItemInstance :type "ItemInstance Object Reference"))
  (returns (`Item Index` :type Integer) (`Inventory Item` :type "/Game/InventorySystem/Types/S_InventoryItem Structure"))
  (for (_array_element _array_index) (`self.InventoryItems`)
    (if (== (`.ItemInstance_7_EF089A1F46A4335E27C140B17A59DF67` (break `/Game/InventorySystem/Types/S_InventoryItem` _array_element)) ItemInstance)
      (return _array_index _array_element)))
  (return -1))

(fn `FindPartialStack`
  (params (ItemDefinition :type "ItemDefinition Class Reference"))
  (returns (ItemIndex :type Integer) (IsFound :type Boolean))
  (for (_array_element _array_index) (`self.InventoryItems`)
    (`/Engine/EditorBlueprintResources/StandardMacros.IsValid` (break `/Game/InventorySystem/Types/S_InventoryItem` _array_element)
      (:`Is Valid`
        (if (and (== (`ItemInstance.ItemDefinition` (break `/Game/InventorySystem/Types/S_InventoryItem` _array_element)) ItemDefinition) (< (`.Count_5_DE33369B4029D74F29A5D9B9116881FD` (break `/Game/InventorySystem/Types/S_InventoryItem` _array_element)) (`/Game/InventorySystem/BFL_InventoryHelpers.GetItemMaxStackCount` ItemDefinition)))
          (return _array_index true)))
      (:`Is Not Valid`
        (return -1 false))))
  (return -1 false))

(fn `GetDropLocation`
  (returns (Location :type "Vector Structure"))
  (bind _returnvalue (`self.GetOwner`))
  (return (+ (`Actor.K2_GetActorLocation` _returnvalue) (* (`Actor.GetActorForwardVector` _returnvalue) 200.0))))

(fn `HandleLoadInventory`
  (bind _savegameobject (message `/Game/SaveSystem/BPI_SaveAndLoadManager.GetSaveGameObject` (`GameplayStatics.GetGameInstance`)))
  (`/Engine/EditorBlueprintResources/StandardMacros.IsValid` _savegameobject
    (:`Is Valid`
      (for _array_element (`/Game/SaveSystem/BP_SaveGame.PlayerInventoryItems` _savegameobject)
        (bind _returnvalue (`|GenericCreateObject` "/Script/ProjectRavenGrub.ItemInstance"))
        (bind (_itemdefinition _count _statsmap) (break `/Game/InventorySystem/Types/S_InventoryItemSnapshot` _array_element))
        (`ItemInstance.Initialize` _returnvalue _itemdefinition _statsmap)
        (`KismetArrayLibrary.Array_Add` (`self.InventoryItems`) (make `/Game/InventorySystem/Types/S_InventoryItem` _returnvalue _count))))))

(fn `HandleSaveInventory`
  (bind _savegameobject (message `/Game/SaveSystem/BPI_SaveAndLoadManager.GetSaveGameObject` (`GameplayStatics.GetGameInstance`)))
  (`/Engine/EditorBlueprintResources/StandardMacros.IsValid` _savegameobject
    (:`Is Valid`
      (bind _playerinventoryitems (`/Game/SaveSystem/BP_SaveGame.PlayerInventoryItems` _savegameobject))
      (`KismetArrayLibrary.Array_Clear` _playerinventoryitems)
      (for _array_element (`self.InventoryItems`)
        (bind (_iteminstance _count) (break `/Game/InventorySystem/Types/S_InventoryItem` _array_element))
        (`KismetArrayLibrary.Array_Add` _playerinventoryitems (make `/Game/InventorySystem/Types/S_InventoryItemSnapshot` (`ItemInstance.ItemDefinition` _iteminstance) _count (`ItemInstance.StatsMap` _iteminstance)))))))

(fn `IsItemEquipped`
  (params (ItemInstance :type "ItemInstance Object Reference"))
  (returns (ReturnValue :type Boolean))
  (bind _returnvalue (`Actor.GetComponentByClass` (`self.GetOwner`) "/Game/EquipmentSystem/BPC_EquipmentManager.BPC_EquipmentManager_C"))
  (`/Engine/EditorBlueprintResources/StandardMacros.IsValid` _returnvalue
    (:`Is Valid`
      (`/Engine/EditorBlueprintResources/StandardMacros.IsValid` (`/Game/EquipmentSystem/BPC_EquipmentManager.FindEquipmentByItemInstance` _returnvalue ItemInstance)
        (:`Is Valid`
          (return true))
        (:`Is Not Valid`
          _)))
    (:`Is Not Valid`
      _))
  (return false))

(fn `RemoveAllItemsOfType`
  (params (ItemDefinition :type "ItemDefinition Class Reference"))
  (bind _inventoryitems (`self.FindAllItems` ItemDefinition))
  (for _array_element _inventoryitems
    (`KismetArrayLibrary.Array_Remove` (`self.InventoryItems`) (`KismetArrayLibrary.Array_Find` (`self.InventoryItems`) _array_element))))

(fn `SetItemCount`
  (params (ItemDefinition :type "ItemDefinition Class Reference") (Count :type Integer))
  (`self.RemoveAllItemsOfType` ItemDefinition)
  (`self.AddItem` (make `/Game/InventorySystem/Types/S_InventoryItemSnapshot` ItemDefinition Count)))

(fn `UseItem`
  (params (SuppressSound :type Boolean) (ItemInstance :type "ItemInstance Object Reference"))
  (returns (Success :type Boolean))
  (bind _returnvalue (`ItemInstance.FindFragmentByClass` ItemInstance "/Script/ProjectRavenGrub.InventoryFragment_Useable"))
  (bind _bconsumeonuse (`InventoryFragment_Useable.bConsumeOnUse` _returnvalue))
  (if (`KismetArrayLibrary.Array_IsNotEmpty` (`self.InventoryItems`))
    (`/Engine/EditorBlueprintResources/StandardMacros.IsValid` _returnvalue
      (:`Is Valid`
        (bind _returnvalue_2 (`InventoryFragment_Useable.Use` _returnvalue (`self.GetOwner`) ItemInstance SuppressSound))
        (if (and _returnvalue_2 _bconsumeonuse)
          (`self.ConsumeItem` (`local.ItemInstance`))
          (`self.OnInventoryChanged`)
          (return true)
          (else
            (`self.OnInventoryChanged`)
            (return _bconsumeonuse))))
      (:`Is Not Valid`
        _)))
  (return false))